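; Coin pickup actor that increments the game mode's coin count and plays a sound, either on direct contact or through the player's magnet power-up.
; Touching the coin collects and destroys it unless already used.
; With MagnetActive, the magnet volume counts it immediately, sets Used and destroys it one second later, while a timeline interpolates it toward the player.
; A two-second delay meant to clear MagnetActive outlasts the coin's destruction.
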(event `self.ReceiveActorBeginOverlap`
  (params (OtherActor :type "Actor Object Reference")))

(event `self.Magnet Collision.OnComponentBeginOverlap`
  (params (OverlappedComponent :type "PrimitiveComponent Object Reference") (OtherActor :type "Actor Object Reference") (OtherComp :type "PrimitiveComponent Object Reference") (OtherBodyIndex :type Integer) (bFromSweep :type Boolean) (SweepResult :type "HitResult Structure (by ref)"))
  (bind _asbp_third_person_character (cast `/Game/Characters/BluePrints/BP_ThirdPersonCharacter` OtherActor))
  (if (`/Game/Characters/BluePrints/BP_ThirdPersonCharacter.Magnet Active` _asbp_third_person_character)
    (`|ExecutionSequence`
      (:`then_0`
        (bind _asbp_third_person_game_mode (cast `/Game/Characters/BluePrints/BP_ThirdPersonGameMode` (`GameplayStatics.GetGameMode`)))
        (`/Engine/EditorBlueprintResources/StandardMacros.IncrementInt` (`/Game/Characters/BluePrints/BP_ThirdPersonGameMode.Coin Var` _asbp_third_person_game_mode)
          (:`  `
            (set `self.Used ` true)
            (`GameplayStatics.SpawnSound2D` "/Game/Runner_Assets/SFX/Pickup_SFX_Cue.Pickup_SFX_Cue" 1.0 1.0 0.0 null)
            (`KismetSystemLibrary.Delay` 1.0)
            (`self.K2_DestroyActor`))))
      (:`then_1`
        (bind (_direction _slide) (`Timeline|MagnetTimeLine` :!via `PlayFromStart`)
          (:`Update`
            (`self.K2_SetActorLocation` (+ _slide (`KismetMathLibrary.VInterpTo` (.location (`self.GetTransform`)) (`self.K2_GetActorLocation` (`GameplayStatics.GetPlayerCharacter` 0)) (`GameplayStatics.GetWorldDeltaSeconds`) 15.0)))
            (`KismetSystemLibrary.Delay` 2.0)
            (set `/Game/Characters/BluePrints/BP_ThirdPersonCharacter.Magnet Active` false _asbp_third_person_character)))))))

(event `self.Coin.OnComponentBeginOverlap`
  (params (OverlappedComponent :type "PrimitiveComponent Object Reference") (OtherActor :type "Actor Object Reference") (OtherComp :type "PrimitiveComponent Object Reference") (OtherBodyIndex :type Integer) (bFromSweep :type Boolean) (SweepResult :type "HitResult Structure (by ref)"))
  (cast `/Game/Characters/BluePrints/BP_ThirdPersonCharacter` OtherActor)
  (bind _asbp_third_person_game_mode (cast `/Game/Characters/BluePrints/BP_ThirdPersonGameMode` (`GameplayStatics.GetGameMode`)))
  (if (not (`self.Used `))
    (set `/Game/Characters/BluePrints/BP_ThirdPersonGameMode.Coin Var` (+ (`/Game/Characters/BluePrints/BP_ThirdPersonGameMode.Coin Var` _asbp_third_person_game_mode) 1) _asbp_third_person_game_mode)
    (`GameplayStatics.SpawnSound2D` "/Game/Runner_Assets/SFX/Pickup_SFX_Cue.Pickup_SFX_Cue" 1.0 1.0 0.0 null)
    (`self.K2_DestroyActor`)))

(fn `UserConstructionScript`)