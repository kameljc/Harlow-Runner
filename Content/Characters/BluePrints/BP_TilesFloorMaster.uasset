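; Master floor tile for a three-lane endless runner, filling its lanes with pipes, boxes, coins or magnets on BeginPlay.
; Each spawn check rolls a fresh random number, and a lane that spawns nothing skips the lanes after it.
; Player overlap makes the game mode spawn another tile and add multiplied score, then destroys this tile after a delay.
; Overlap also scales walk speed, but equal clamp bounds pin it at 2000.
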(event `self.ReceiveBeginPlay`
  (`self.Spawn Obstacles`))

(event `self.Box.OnComponentBeginOverlap`
  (params (OverlappedComponent :type "PrimitiveComponent Object Reference") (OtherActor :type "Actor Object Reference") (OtherComp :type "PrimitiveComponent Object Reference") (OtherBodyIndex :type Integer) (bFromSweep :type Boolean) (SweepResult :type "HitResult Structure (by ref)"))
  (cast `/Game/Characters/BluePrints/BP_ThirdPersonCharacter` OtherActor)
  (bind _asbp_third_person_game_mode (cast `/Game/Characters/BluePrints/BP_ThirdPersonGameMode` (`GameplayStatics.GetGameMode`)))
  (`/Game/Characters/BluePrints/BP_ThirdPersonGameMode.TileSpawner` _asbp_third_person_game_mode)
  (bind _asbp_third_person_game_mode_2 (cast `/Game/Characters/BluePrints/BP_ThirdPersonGameMode` (`GameplayStatics.GetGameMode`)))
  (`self.Calculating Score Over time` _asbp_third_person_game_mode_2 _asbp_third_person_game_mode_2 _asbp_third_person_game_mode_2)
  (bind _asbp_third_person_character (cast `/Game/Characters/BluePrints/BP_ThirdPersonCharacter` (`GameplayStatics.GetPlayerCharacter` 0)))
  (`self.Increasing Speed Over Time` _asbp_third_person_character)
  (`KismetSystemLibrary.Delay` 0.6)
  (`self.K2_DestroyActor`))

(fn `Calculating Score Over time`
  (params (self2 :type "/Game/Characters/BluePrints/BP_ThirdPersonGameMode Object Reference") (self3 :type "/Game/Characters/BluePrints/BP_ThirdPersonGameMode Object Reference") (self4 :type "/Game/Characters/BluePrints/BP_ThirdPersonGameMode Object Reference"))
  (set `/Game/Characters/BluePrints/BP_ThirdPersonGameMode.Current Point ` (+ (* 1 (`/Game/Characters/BluePrints/BP_ThirdPersonGameMode.Point Multiplier` self4)) (`/Game/Characters/BluePrints/BP_ThirdPersonGameMode.Current Point ` self3)) self2))

(fn `Increasing Speed Over Time`
  (params (self2 :type "Character Object Reference"))
  (bind _charactermovement (`Character.CharacterMovement` self2))
  (set `CharacterMovementComponent.MaxWalkSpeed` (`KismetMathLibrary.FClamp` (* (`CharacterMovementComponent.MaxWalkSpeed` _charactermovement) 1.01) 2000.0 2000.0) _charactermovement))

(fn `Spawn Obstacles`
  (bind _returnvalue (`KismetMathLibrary.RandomFloatInRange` 0.0 1.0))
  (bind _returnvalue_2 (`KismetMathLibrary.RandomFloatInRange` 0.0 1.0))
  (bind _returnvalue_3 (`KismetMathLibrary.RandomFloatInRange` 0.0 1.0))
  (bind _returnvalue_4 (`SceneComponent.K2_GetComponentToWorld` (`self.Lane0`)))
  (bind _returnvalue_5 (`SceneComponent.K2_GetComponentToWorld` (`self.Lane1`)))
  (bind _returnvalue_6 (`SceneComponent.K2_GetComponentToWorld` (`self.Lane2`)))
  ;[1 1 1] Spawn Obstacle at Lane 0
  (if (`KismetMathLibrary.InRange_FloatFloat` _returnvalue_2 0.0 0.4)
    (`|SpawnActorFromClass` "/Game/Characters/BluePrints/BP_Obstacle_Pipe.BP_Obstacle_Pipe_C" _returnvalue_4 "Undefined" "OverrideRootScale" null null)
    ;[1 1 1] Lane 1
    (if (`KismetMathLibrary.InRange_FloatFloat` _returnvalue_3 0.0 0.4) :!label _label
      (`|SpawnActorFromClass` "/Game/Characters/BluePrints/BP_Obstacle_Pipe.BP_Obstacle_Pipe_C" _returnvalue_5 "Undefined" "OverrideRootScale" null null)
      ;[1 1 1] Lane2
      (if (`KismetMathLibrary.InRange_FloatFloat` _returnvalue 0.0 0.4) :!label _label_2
        (`|SpawnActorFromClass` "/Game/Characters/BluePrints/BP_Obstacle_Pipe.BP_Obstacle_Pipe_C" _returnvalue_6 "Undefined" "OverrideRootScale" null null)
        (elif (`KismetMathLibrary.InRange_FloatFloat` _returnvalue 0.4 0.5)
          (`|SpawnActorFromClass` "/Game/Characters/BluePrints/BP_Obstacle_Box.BP_Obstacle_Box_C" _returnvalue_6 "Undefined" "OverrideRootScale" null null)
          (elif (`KismetMathLibrary.InRange_FloatFloat` _returnvalue 0.5 0.95)
            (`|SpawnActorFromClass` "/Game/Characters/BluePrints/BP_Coin_PickUp.BP_Coin_PickUp_C" _returnvalue_6 "Undefined" "OverrideRootScale" null null)
            (elif (`KismetMathLibrary.InRange_FloatFloat` _returnvalue 0.95)
              (`|SpawnActorFromClass` "/Game/Characters/BluePrints/BP_Magnet.BP_Magnet_C" _returnvalue_6 "Undefined" "OverrideRootScale" null null)))))
      (elif (`KismetMathLibrary.InRange_FloatFloat` _returnvalue_3 0.4 0.5)
        (`|SpawnActorFromClass` "/Game/Characters/BluePrints/BP_Obstacle_Box.BP_Obstacle_Box_C" _returnvalue_5 "Undefined" "OverrideRootScale" null null)
        (goto _label_2)
        (elif (`KismetMathLibrary.InRange_FloatFloat` _returnvalue_3 0.5 0.95)
          (`|SpawnActorFromClass` "/Game/Characters/BluePrints/BP_Coin_PickUp.BP_Coin_PickUp_C" _returnvalue_5 "Undefined" "OverrideRootScale" null null)
          (goto _label_2)
          (elif (`KismetMathLibrary.InRange_FloatFloat` _returnvalue_3 0.95)
            (`|SpawnActorFromClass` "/Game/Characters/BluePrints/BP_Magnet.BP_Magnet_C" _returnvalue_5 "Undefined" "OverrideRootScale" null null)
            (goto _label_2)))))
    (elif (`KismetMathLibrary.InRange_FloatFloat` _returnvalue_2 0.4 0.5)
      (`|SpawnActorFromClass` "/Game/Characters/BluePrints/BP_Obstacle_Box.BP_Obstacle_Box_C" _returnvalue_4 "Undefined" "OverrideRootScale" null null)
      (goto _label)
      (elif (`KismetMathLibrary.InRange_FloatFloat` _returnvalue_2 0.5 0.95)
        (`|SpawnActorFromClass` "/Game/Characters/BluePrints/BP_Coin_PickUp.BP_Coin_PickUp_C" _returnvalue_4 "Undefined" "OverrideRootScale" null null)
        (goto _label)
        (elif (`KismetMathLibrary.InRange_FloatFloat` _returnvalue_2 0.95 1.0)
          (`|SpawnActorFromClass` "/Game/Characters/BluePrints/BP_Magnet.BP_Magnet_C" _returnvalue_4 "Undefined" "OverrideRootScale" null null)
          (goto _label))))))

(fn `UserConstructionScript`)